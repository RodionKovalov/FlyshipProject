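; A-10 aircraft pawn that layers flight physics, animation, cockpit instruments and effects on a parent aircraft class.
; The authority enables mesh physics, and Tick applies each FlyMovementComponent surface's force and torque as acceleration.
; Tick also feeds suspension, wheel, gear and control-surface values to the AnimInstance, and flight data to the HUD mesh and gauges.
; Thrust drives engine pitch and distortion Niagara, while first-person view applies a cabin sound mix.
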(event `self.CameraAction`
  (`parent.CameraAction`)
  (`self.ToogleCabinSound`))

(event `self.ReceiveBeginPlay`
  (`parent.ReceiveBeginPlay`)
  (`|ExecutionSequence`
    (:`then_0`
      (`/Engine/EditorBlueprintResources/ActorMacros.Switch Has Authority`
        (:`Authority`
          (`PrimitiveComponent.SetSimulatePhysics` (`self.SkeletalMesh`) true))))
    (:`then_1`
      (bind _asbpa_west_attack_a10 (cast `/Game/VigilanteContent/Vehicles/West_Attack_A10/BPA_West_Attack_A10` (`SkeletalMeshComponent.GetAnimInstance` (`self.SkeletalMesh`))))
      (set `self.AnimInstance` _asbpa_west_attack_a10))))

(event `self.PlayDeadEffects`
  (`GameplayStatics.PopSoundMixModifier` "/Game/AirCraft/Blueprints/Sounds/CabinClassMix.CabinClassMix"))

(event `self.ReceiveTick`
  (params (DeltaSeconds :type "Float (single-precision)"))
  (bind _skeletalmesh (`self.SkeletalMesh`))
  (`parent.ReceiveTick` DeltaSeconds)
  (`|ExecutionSequence`
    (:`then_0`
      (`self.UpdateSound`)
      (`self.UpdateSuspension`)
      (`self.UpdateRotationWheels`)
      (`self.UpdateFlaps`)
      (`self.Update WheelsRetract`)
      (`self.UpdateHUD`)
      (`self.Update Panels`)
      (`self.UpdateDistortionEffects`))
    (:`then_1`
      (if (`SceneComponent.IsSimulatingPhysics` (`self.SkeletalMesh`) "None")
        (for _array_element (`FlyMovementComponent.Surfaces` (`self.FlyMovementComponent`))
          (bind _returnvalue (`SurfaceWind.CalculateForceAndTorque` _array_element))
          (bind (_p _q) (break `BiVector` _returnvalue))
          (`PrimitiveComponent.AddForce` _skeletalmesh _p "None" true)
          (`PrimitiveComponent.AddTorqueInDegrees` _skeletalmesh (* _q 0.01) "None" true))))))

(fn `ToogleCabinSound`
  (if (`ActorComponent.IsActive` (`self.FirstPersonCamera`))
    (`GameplayStatics.SetSoundMixClassOverride` "/Game/AirCraft/Blueprints/Sounds/CabinClassMix.CabinClassMix" "/Game/AirCraft/Blueprints/Sounds/SFX_SoundClass.SFX_SoundClass" 1.0 1.0 0.1)
    (`/Engine/EditorBlueprintResources/StandardMacros.DoOnce` false :!label _label
      (:`Completed`
        (`GameplayStatics.PushSoundMixModifier` "/Game/AirCraft/Blueprints/Sounds/CabinClassMix.CabinClassMix")))
    (else
      (`GameplayStatics.PopSoundMixModifier` "/Game/AirCraft/Blueprints/Sounds/CabinClassMix.CabinClassMix")
      (goto _label :!via `Reset`))))

(fn `Update Distortion Parameters`)

(fn `Update Panels`
  (bind (_returnvalue_x _returnvalue_y _returnvalue_z) (`KismetMathLibrary.BreakVector` (`self.GetVelocity`)))
  (`MaterialInstanceDynamic.SetScalarParameterValue` (`/Game/AirCraft/Blueprints/AircraftPanels/Indicator.MaterialInstance` (`self.IASPanel`)) "Speed" (/ (`KismetMathLibrary.VSize` (`self.GetVelocity`)) 51.444))
  (`MaterialInstanceDynamic.SetScalarParameterValue` (`/Game/AirCraft/Blueprints/AircraftPanels/Indicator.MaterialInstance` (`self.VerticalSpeedIndicator`)) "Speed" _returnvalue_z))

(fn `Update WheelsRetract`
  (bind _animinstance (`self.AnimInstance`))
  (bind _alphawheels (`self.AlphaWheels`))
  (set `self.AlphaWheels` (`KismetMathLibrary.FInterpTo` (`self.AlphaWheels`) (`KismetMathLibrary.SelectFloat` 0.0 1.0 (`self.bActiveWheels`)) (`self.DeltaTimeSeconds`) (`self.InterpSpeedAlphaWheels`)))
  (set `/Game/VigilanteContent/Vehicles/West_Attack_A10/BPA_West_Attack_A10.FrontWheelRetract` _alphawheels _animinstance)
  (set `/Game/VigilanteContent/Vehicles/West_Attack_A10/BPA_West_Attack_A10.RearWheelLRetract` _alphawheels _animinstance)
  (set `/Game/VigilanteContent/Vehicles/West_Attack_A10/BPA_West_Attack_A10.RearWheelRRetract` _alphawheels _animinstance))

(fn `UpdateDistortionEffects`
  (`ActorComponent.SetActive` (`self.DistorionL_Niagara`) (> (`FlyMovementComponent.ThrustSpeed` (`self.FlyMovementComponent`)) 0.0) false)
  (`ActorComponent.SetActive` (`self.DistorionR_Niagara`) (> (`FlyMovementComponent.ThrustSpeed` (`self.FlyMovementComponent`)) 0.0) false)
  (`self.Update Distortion Parameters`))

(fn `UpdateFlaps`
  (bind _animinstance (`self.AnimInstance`))
  (bind _returnvalue (* (`SurfaceWind.FlapAngle` (`self.BP_StabilizerLSurfaceWind`)) 15.0))
  (bind _returnvalue_2 (* (`SurfaceWind.FlapAngle` (`self.BP_WindRSurfaceWind`)) 15.0))
  (bind _returnvalue_3 (* (`KismetMathLibrary.FClamp` (`SurfaceWind.FlapAngle` (`self.BP_WindR2SurfaceWind`)) -1.0) 15.0))
  (bind _returnvalue_4 (* _returnvalue_3 -1.0))
  (set `/Game/VigilanteContent/Vehicles/West_Attack_A10/BPA_West_Attack_A10.RuddersAngle` (* (`SurfaceWind.FlapAngle` (`self.BP_Tail_VLSurfaceWind`)) 15.0) _animinstance)
  (set `/Game/VigilanteContent/Vehicles/West_Attack_A10/BPA_West_Attack_A10.InnerFlapsAngle` 0.0 _animinstance)
  (set `/Game/VigilanteContent/Vehicles/West_Attack_A10/BPA_West_Attack_A10.AileronLTop` _returnvalue_3 _animinstance)
  (set `/Game/VigilanteContent/Vehicles/West_Attack_A10/BPA_West_Attack_A10.AileronRTop` _returnvalue_4 _animinstance)
  (set `/Game/VigilanteContent/Vehicles/West_Attack_A10/BPA_West_Attack_A10.AileronLBottom` _returnvalue_3 _animinstance)
  (set `/Game/VigilanteContent/Vehicles/West_Attack_A10/BPA_West_Attack_A10.AileronRBottom` _returnvalue_4 _animinstance)
  (set `/Game/VigilanteContent/Vehicles/West_Attack_A10/BPA_West_Attack_A10.ElevatorLAngle` _returnvalue _animinstance)
  (set `/Game/VigilanteContent/Vehicles/West_Attack_A10/BPA_West_Attack_A10.ElevatorRAngle` _returnvalue _animinstance)
  (set `/Game/VigilanteContent/Vehicles/West_Attack_A10/BPA_West_Attack_A10.InnerFlapsAngle` _returnvalue_2 _animinstance)
  (set `/Game/VigilanteContent/Vehicles/West_Attack_A10/BPA_West_Attack_A10.OuterFlapsAngle` _returnvalue_2 _animinstance))

(fn `UpdateHUD`
  (bind _deltatimeseconds (`self.DeltaTimeSeconds`))
  (bind _x (.x (`KismetMathLibrary.InverseTransformDirection` (`self.GetTransform`) (`self.GetVelocity`))))
  (bind _y (.y (`KismetMathLibrary.InverseTransformDirection` (`self.GetTransform`) (`self.GetVelocity`))))
  (set `self.Alt` (* (.z (`self.K2_GetActorLocation`)) 0.032808))
  (set `self.Speed` (* _x 0.019438))
  ;[1 1 1] Call Event to update Hud Mesh
  (`/Game/AirCraft/AircraftHud/Blueprints/BP_HudMesh.Hud_Update_Event` (`self.BP_HudMesh`) (.roll (`self.K2_GetActorRotation`)) (.pitch (`self.K2_GetActorRotation`)) (.yaw (`self.K2_GetActorRotation`)) (`self.Alt`) (`self.Speed`) (/ (/ (- (`self.Speed`) (`self.PrevSpeed`)) _deltatimeseconds) 20.0) (/ (/ (- (`self.Alt`) (`self.PrevAlt`)) _deltatimeseconds) 20.0) (`KismetMathLibrary.FClamp` (/ _y 100.0) -1.0) (`KismetMathLibrary.FClamp` (`KismetMathLibrary.DegAtan2` (.z (`KismetMathLibrary.InverseTransformDirection` (`self.GetTransform`) (`self.GetVelocity`))) _x) -90.0 90.0) (`KismetMathLibrary.FClamp` (`KismetMathLibrary.DegAtan2` _y _x) -90.0 90.0))
  (set `self.PrevSpeed` (`self.Speed`))
  (set `self.PrevAlt` (`self.Alt`)))

(fn `UpdateRotationWheels`
  (bind _animinstance (`self.AnimInstance`))
  (for _array_element (`VehicleComponent.WheelsRef` (`self.VehicleComponent`))
    (switch `name` (`Wheel.BoneName` _array_element)
      (:`WheelF`
        (bind _wheellinearvelocity_x (`KismetMathLibrary.BreakVector` (`Wheel.WheelLinearVelocity` _array_element)))
        (bind _returnvalue (`KismetMathLibrary.RadiansToDegrees` (/ _wheellinearvelocity_x (`Wheel.WheelRadius` _array_element))))
        (set `/Game/VigilanteContent/Vehicles/West_Attack_A10/BPA_West_Attack_A10.WheelFRotationSpeed` _returnvalue _animinstance))
      (:`WheelL`
        (set `/Game/VigilanteContent/Vehicles/West_Attack_A10/BPA_West_Attack_A10.WheelLRotationSpeed` _returnvalue _animinstance))
      (:`WheelR`
        (set `/Game/VigilanteContent/Vehicles/West_Attack_A10/BPA_West_Attack_A10.WheelRRotationSpeed` _returnvalue _animinstance)))))

(fn `UpdateSound`
  (bind _flymovementcomponent (`self.FlyMovementComponent`))
  (`AudioComponent.SetFloatParameter` (`self.Audio`) "Pitch_Alpha" (/ (`FlyMovementComponent.ThrustSpeed` _flymovementcomponent) (`FlyMovementComponent.MaxThrustSpeed` _flymovementcomponent))))

(fn `UpdateSuspension`
  (bind _animinstance (`self.AnimInstance`))
  (for _array_element (`VehicleComponent.WheelsRef` (`self.VehicleComponent`))
    (switch `name` (`Wheel.BoneName` _array_element)
      (:`WheelF`
        (bind _suspnesiontravel (`Wheel.SuspnesionTravel` _array_element))
        (bind _returnvalue (`KismetMathLibrary.MapRangeClamped` (`Wheel.Length` _array_element) (+ (`Wheel.SuspensionRestLength` _array_element) _suspnesiontravel) 0.0 0.0 (+ _suspnesiontravel (`Wheel.WheelRadius` _array_element))))
        (set `/Game/VigilanteContent/Vehicles/West_Attack_A10/BPA_West_Attack_A10.Rear WheelFSuspension` _returnvalue _animinstance))
      (:`WheelL`
        (set `/Game/VigilanteContent/Vehicles/West_Attack_A10/BPA_West_Attack_A10.Rear WheelLSuspension` _returnvalue _animinstance))
      (:`WheelR`
        (set `/Game/VigilanteContent/Vehicles/West_Attack_A10/BPA_West_Attack_A10.Rear WheelRSuspension` _returnvalue _animinstance)))))

(fn `UserConstructionScript`
  (`parent.UserConstructionScript`))
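; BP_SurfaceWind is an aircraft Blueprint whose own graph currently adds no active behavior beyond its parent's Tick.
; Tick calls the parent, then checks for a valid owner with network authority, but that branch leads to nothing.
; A disconnected chain would apply the result of CalculateForceAndTorque to the mesh as acceleration-based force and scaled-down torque, but it never executes.
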(event `self.ReceiveTick`
  (params (DeltaSeconds :type "Float (single-precision)"))
  (bind _owner (`self.Owner`))
  (`parent.ReceiveTick` DeltaSeconds)
  (`/Engine/EditorBlueprintResources/StandardMacros.IsValid` _owner
    (:`Is Valid`
      (if (`Actor.HasAuthority` _owner)
        _))))
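; Main player controller that caches the game's MainHUD and handles character restart and menu input.
; Restart kills the controlled pawn with huge damage, running locally and, on clients, also through a server event.
; The Q key opens the pause menu, and the PlayerList action shows the player list while held.
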(event `self.ReceiveBeginPlay`
  (`parent.ReceiveBeginPlay`)
  (bind _asmain_hud (cast `/Game/AirCraft/Blueprints/Widgets/MainHUD` (`self.GetHUD`)))
  (set `self.HUD` _asmain_hud))

(event `ClientRestartCharacter`
  (`self.RestartCharacter`)
  (if (not (`self.HasAuthority`))
    (`self.ServerRestartCharacter`)))

(event `ServerRestartCharacter`
  (`self.RestartCharacter`))

(event `Key|Q`
  (params (Key :type "Key Structure"))
  (:`Pressed`
    (bind _hud (`self.HUD`)
      (:`then`
        (`/Game/AirCraft/Blueprints/Widgets/MainHUD.SetPauseMenu` _hud true))
      (:`else`))))

(event `InputAction|PlayerList`
  (params (Key :type "Key Structure"))
  (:`Pressed`
    (bind _hud (`self.HUD`)
      (:`then`
        (`/Game/AirCraft/Blueprints/Widgets/MainHUD.SetPlayerList` _hud true))
      (:`else`)))
  (:`Released`
    (bind _hud_2 (`self.HUD`)
      (:`then`
        (`/Game/AirCraft/Blueprints/Widgets/MainHUD.SetPlayerList` _hud_2 false))
      (:`else`))))

(fn `RestartCharacter`
  (`GameplayStatics.ApplyDamage` (`self.K2_GetPawn`) 9999999.0 (`self.GetInstigatorController`) self))

(fn `UserConstructionScript`)
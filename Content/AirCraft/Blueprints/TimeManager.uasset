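; TimeManager drives a day/night cycle by pitching a directional light source each tick at a configurable Speed and refreshing the sky sphere's sun direction.
; The light's pitch picks the branch: a positive pitch up to the range limit runs NichtLighting (night), anything else runs DayLighting.
; Both functions slowly interpolate sky light intensity, fog density and sun intensity toward their own targets using a scaled-down delta time.
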(event `self.ReceiveTick`
  (params (DeltaSeconds :type "Float (single-precision)"))
  (bind _lightcomponent (`Light.LightComponent` (`self.LightSource`)))
  (bind (_returnvalue_roll _returnvalue_pitch) (`KismetMathLibrary.BreakRotator` (`SceneComponent.K2_GetComponentRotation` _lightcomponent)))
  (`SceneComponent.K2_AddWorldRotation` _lightcomponent (`KismetMathLibrary.MakeRotator` 0.0 (* DeltaSeconds (`self.Speed`))) false false)
  (`/Engine/EngineSky/BP_Sky_Sphere.UpdateSunDirection` (`self.SkyShere`))
  (if (`KismetMathLibrary.InRange_FloatFloat` _returnvalue_pitch 0.0 100.0)
    (`self.NichtLighting` DeltaSeconds)
    (else
      (`self.DayLighting` DeltaSeconds))))

(fn `DayLighting`
  (params (Delta :type "Float (double-precision)"))
  (bind _returnvalue (/ Delta 64.0))
  (bind _lightcomponent (`Light.LightComponent` (`self.LightSource`)))
  (bind _lightcomponent_2 (`SkyLight.LightComponent` (`self.SkyLight`)))
  (bind _component (`ExponentialHeightFog.Component` (`self.Fog`)))
  (`SkyLightComponent.SetIntensity` _lightcomponent_2 (`KismetMathLibrary.FInterpTo` (`LightComponentBase.Intensity` _lightcomponent_2) 1.0 _returnvalue 8.0))
  (`ExponentialHeightFogComponent.SetFogDensity` _component (`KismetMathLibrary.FInterpTo` (`ExponentialHeightFogComponent.FogDensity` _component) 0.01 _returnvalue 8.0))
  (`LightComponent.SetIntensity` _lightcomponent (`KismetMathLibrary.FInterpTo` (`LightComponentBase.Intensity` _lightcomponent) 2.75 _returnvalue 8.0)))

(fn `NichtLighting`
  (params (Delta :type "Float (double-precision)"))
  (bind _returnvalue (/ Delta 64.0))
  (bind _lightcomponent (`Light.LightComponent` (`self.LightSource`)))
  (bind _lightcomponent_2 (`SkyLight.LightComponent` (`self.SkyLight`)))
  (bind _component (`ExponentialHeightFog.Component` (`self.Fog`)))
  (`SkyLightComponent.SetIntensity` _lightcomponent_2 (`KismetMathLibrary.FInterpTo` (`LightComponentBase.Intensity` _lightcomponent_2) 0.0 _returnvalue 8.0))
  (`ExponentialHeightFogComponent.SetFogDensity` _component (`KismetMathLibrary.FInterpTo` (`ExponentialHeightFogComponent.FogDensity` _component) 0.0 _returnvalue 8.0))
  (`LightComponent.SetIntensity` _lightcomponent (`KismetMathLibrary.FInterpTo` (`LightComponentBase.Intensity` _lightcomponent) 0.01 _returnvalue 8.0)))

(fn `UserConstructionScript`)